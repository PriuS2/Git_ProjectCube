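; BP_ConnectionLine is a puzzle connection line that draws a spline-based mesh and relays on/off signals to linked actors.
; The construction script builds one spline mesh per segment from point locations and tangents, and briefly draws blue debug lines to each valid ConnectedActor.
; SendMessage forwards the OnOff state to every entry in ConnectedActor.
; Unwired construction nodes for additional oriented mesh pieces never run.
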(event EventSendMessage
  (params (On/Off :type Boolean))
  (for _array_element (Variables|Default|GetConnectedActor)
    (Class|BISendMessage|SendMessage(Message) _array_element On/Off)))

(fn ConstructionScript
  (bind _spline (Variables|Default|GetSpline))
  (for _index (range 0 (- (Spline|GetNumberOfSplinePoints (Variables|Default|GetSpline)) 2))
    (bind _returnvalue (AddComponent|AddSplineMeshComponent false))
    (Class|SceneComponent|Attachto _returnvalue (Variables|Default|GetDefaultSceneRoot) "None" "KeepRelativeOffset" true)
    (SplineMesh|SetStartandEnd _returnvalue (.Location (Spline|GetLocationandTangentatSplinePoint _spline _index "Local")) (.Tangent (Spline|GetLocationandTangentatSplinePoint _spline _index "Local")) (.Location (Spline|GetLocationandTangentatSplinePoint _spline (+ _index 1) "Local")) (.Tangent (Spline|GetLocationandTangentatSplinePoint _spline (+ _index 1) "Local")) true :!class /Script/Engine.SplineMeshComponent))
  (for _array_element (Variables|Default|GetConnectedActor)
    (Utilities|IsValid _array_element
      (:Is%20Valid
        (Rendering|Debug|DrawDebugLine (Transformation|GetActorLocation) (Transformation|GetActorLocation _array_element) "(R=0.000000,G=0.033423,B=1.000000,A=1.000000)" 0.1 5.0)))))