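; Puzzle lever switch that turns connected actors on or off based on how far its Handle child actor is rotated.
; It stores the handle's rotation one second after BeginPlay, and Tick compares the pitch drop from it against RotateAngle.
; Two DoOnce gates that reset each other send true or false messages to every ConnectedActor only when the state flips, with On/Off debug prints.
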(event EventBeginPlay
  (Utilities|FlowControl|Delay 1.0)
  (Variables|Default|SetInitRotation (Transformation|GetActorRotation (Variables|/Script/Engine.ChildActorComponent|GetChildActor (Variables|Default|GetHandle)))))

(event Collision|EventActorBeginOverlap
  (params (OtherActor :type Actor%20Object%20Reference)))

(event EventTick
  (params (DeltaSeconds :type Float%20%28single-precision%29))
  (if (> (- (.pitch (Variables|Default|GetInitRotation)) (.pitch (Transformation|GetActorRotation (Variables|/Script/Engine.ChildActorComponent|GetChildActor (Variables|Default|GetHandle))))) (Variables|Default|GetRotateAngle))
    (Utilities|FlowControl|DoOnce false :!label _label
      (:Completed
        (for _array_element (Variables|Default|GetConnectedActor)
          (Class|BISendMessage|SendMessage(Message) _array_element true))
        (Utilities|FlowControl|Sequence
          (:then_0
            (goto _label_2 Reset))
          (:then_1
            (Development|PrintString "On")))))
    (else
      (Utilities|FlowControl|DoOnce false :!label _label_2
        (:Completed
          (for _array_element_2 (Variables|Default|GetConnectedActor)
            (Class|BISendMessage|SendMessage(Message) _array_element_2 false))
          (Utilities|FlowControl|Sequence
            (:then_0
              (goto _label Reset))
            (:then_1
              (Development|PrintString "Off"))))))))

(fn ConstructionScript)