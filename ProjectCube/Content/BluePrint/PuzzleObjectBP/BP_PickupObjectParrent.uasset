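; Base pickup puzzle object that BP_MotionController grabs and drops via attachment, a physics handle, or a mixed mode.
; BeginPlay forces physics-handle grabbing when the player is not FirstPersonCharacter.
; Mixed mode attaches, switches to the handle on overlap, and has a lerp-and-reattach path gated by a hit time whose update is disconnected.
; Physics-handle and mixed modes auto-drop when the pivot strays too far from the controller.
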(event OnComponentHit(StaticMeshComponent)
  (params (HitComponent :type Primitive%20Component%20Object%20Reference) (OtherActor :type Actor%20Object%20Reference) (OtherComp :type Primitive%20Component%20Object%20Reference) (NormalImpulse :type Vector :default "0, 0, 0") (Hit :type Hit%20Result%20Structure%20%28by%20ref%29)))

(event Custom|OpenDoOnceGates
  (Utilities|FlowControl|Sequence
    (:then_0
      (Utilities|FlowControl|DoOnce false) ; enters at Reset
    )
    (:then_1
      (Utilities|FlowControl|DoOnce false) ; enters at Reset
    )))

(event EventTick
  (params (DeltaSeconds :type Float%20%28single-precision%29))
  (bind _staticmeshcomponent (Variables|Debug|GetStaticMeshComponent))
  (switch Utilities|FlowControl|Switch|SwitchonGrabMethodEnum (Variables|Default|GetGrabMethod)
    (:NewEnumerator1
      (CallFunction|DropifLostConnection) ; 컨트롤러와 mesh가 일정거리이상되면 Disconnect 됨
    )
    (:NewEnumerator2
      (CallFunction|DropifLostConnection)
      (if (Utilities|IsValid (Variables|Default|GetMC))
        (bind _returnvalue (Class|KismetSystemLibrary|ComponentOverlapComponents _staticmeshcomponent (Transformation|GetWorldTransform _staticmeshcomponent) (Utilities|Array|MakeArray "ObjectTypeQuery1" "ObjectTypeQuery2" "ObjectTypeQuery4" "ObjectTypeQuery7") 0 (Variables|Default|GetActorToIgnore)))
        (if _returnvalue
          (Utilities|FlowControl|DoOnce false :!label _label
            (:Completed
              (CallFunction|DropAttachto)
              (CallFunction|GrabPhysicsHandle)
              (goto _label_2 Reset)))
          (elif (< (- (Utilities|Time|GetGameTimeinSeconds) (Variables|Default|GetHitTime)) 0.0)
            (if (> (Variables|Default|GetLocationAlpha) 1.0)
              (Utilities|FlowControl|DoOnce false :!label _label_2
                (:Completed
                  (CallFunction|DropPhysicsHandle)
                  (CallFunction|GrabAttachto)
                  (goto _label Reset)))
              (else
                (Variables|Default|SetLocationAlpha (+ (Variables|Default|GetLocationAlpha) (* (Utilities|Time|GetWorldDeltaSeconds) 1e+01)))
                (Transformation|SetWorldLocationAndRotation (Variables|Debug|GetStaticMeshComponent) (.location (Math|Transform|Lerp(Transform) (Transformation|GetWorldTransform (Variables|Debug|GetStaticMeshComponent)) (Utilities|GetWorldPickupTransform) (Variables|Default|GetLocationAlpha))) (.rotation (Math|Transform|Lerp(Transform) (Transformation|GetWorldTransform (Variables|Debug|GetStaticMeshComponent)) (Utilities|GetWorldPickupTransform) (Variables|Default|GetLocationAlpha))) false false)))))))))

(event EventBeginPlay
  (bind _outactors (Actor|GetAllActorsOfClass "/Game/BluePrint/VirtualRealityBP/BP_MotionController.BP_MotionController_C"))
  (Variables|Default|SetActorToIgnore _outactors)
  (Utilities|FlowControl|Delay 1.0)
  (Utilities|Casting|CastToFirstPersonCharacter (Game|GetPlayerCharacter 0)
    (:CastFailed
      (Variables|Default|SetGrabMethod "NewEnumerator1"))))

(event EventPickup
  (params (MC :type Scene%20Component%20Object%20Reference) (PH :type Physics%20Handle%20Component%20Object%20Reference))
  ;[1 1 1] PickUp
  (Utilities|FlowControl|Sequence
    (:then_0
      (Utilities|IsValid (Variables|Default|GetMC)
        (:Is%20Valid
          (CallFunction|Drop))))
    (:then_1
      (Variables|Default|SetMC MC)
      (Variables|Default|SetPH PH))
    (:then_2
      (Transformation|SetWorldLocation (Variables|Default|GetPivot) (Transformation|GetWorldLocation (Variables|Default|GetMC)) false false))
    (:then_3
      (switch Utilities|FlowControl|Switch|SwitchonGrabMethodEnum (Variables|Default|GetGrabMethod)
        (:NewEnumerator0
          (CallFunction|GrabAttachto))
        (:NewEnumerator1
          (CallFunction|GrabPhysicsHandle))
        (:NewEnumerator2
          (CallFunction|GrabMixedMode))))))

(event EventDrop
  ;[1 1 1] Drop
  (Utilities|FlowControl|Sequence
    (:then_0
      (switch Utilities|FlowControl|Switch|SwitchonGrabMethodEnum (Variables|Default|GetGrabMethod)
        (:NewEnumerator0
          (CallFunction|DropAttachto))
        (:NewEnumerator1
          (CallFunction|DropPhysicsHandle))
        (:NewEnumerator2
          (CallFunction|DropMixedMode))))
    (:then_1
      (Variables|Default|SetMC 0)
      (Variables|Default|SetPH 0))))

(fn ConstructionScript)

(fn GrabAttachto
  (bind _returnvalue (Utilities|GetWorldPickupTransform))
  (Collision|SetCollisionObjectType (Variables|Debug|GetStaticMeshComponent) "ECC_PhysicsBody")
  (Physics|SetEnableGravity (Variables|Debug|GetStaticMeshComponent) false)
  (Physics|SetSimulatePhysics (Variables|Debug|GetStaticMeshComponent) false)
  (if (Variables|Default|GetIsGrabbed)
    (Transformation|SetWorldLocationAndRotation (Variables|Debug|GetStaticMeshComponent) (.location _returnvalue) (.rotation _returnvalue) false false))
  (Transformation|AttachComponentToComponent (VehicleSound|GetRootComponent) (Variables|Default|GetMC) "None" "KeepWorld" "KeepWorld" "KeepWorld" false)
  (if (not (Variables|Default|GetIsGrabbed))
    (Variables|Default|SetRelativePickupOffset (Utilities|GetRelativePickupTransform))))

(fn GrabPhysicsHandle
  (bind _mc (Variables|Default|GetMC))
  (bind _returnvalue (Transformation|GetWorldTransform _mc))
  (Physics|Components|PhysicsHandle|GrabComponentatLocationwithRotation (Variables|Default|GetPH) (Variables|Debug|GetStaticMeshComponent) "None" (.location _returnvalue) (.rotation _returnvalue))
  (Physics|SetEnableGravity (Variables|Debug|GetStaticMeshComponent) false)
  (Physics|SetSimulatePhysics (Variables|Debug|GetStaticMeshComponent) true)
  (Collision|SetCollisionObjectType (Variables|Debug|GetStaticMeshComponent) "ECC_PhysicsBody")
  (Variables|Default|SetLocationAlpha 0.0))

(fn DropAttachto
  (Physics|SetSimulatePhysics (Variables|Debug|GetStaticMeshComponent) true)
  (Transformation|DetachFromActor "KeepWorld" "KeepWorld" "KeepWorld")
  (Physics|SetEnableGravity (Variables|Debug|GetStaticMeshComponent) true)
  (Physics|SetSimulatePhysics (Variables|Debug|GetStaticMeshComponent) true))

(fn DropPhysicsHandle
  (Physics|Components|PhysicsHandle|ReleaseComponent (Variables|Default|GetPH))
  (Physics|SetEnableGravity (Variables|Debug|GetStaticMeshComponent) true))

(fn GrabMixedMode
  (Collision|SetCollisionResponsetoChannel (Variables|Debug|GetStaticMeshComponent) "ECC_Pawn" "ECR_Ignore")
  (CallFunction|GrabAttachto)
  (Variables|Default|SetIsGrabbed true)
  (CallFunction|OpenDoOnceGates))

(fn DropMixedMode
  (Variables|Default|SetIsGrabbed false)
  (CallFunction|DropAttachto)
  (CallFunction|DropPhysicsHandle)
  (Collision|SetCollisionObjectType (Variables|Debug|GetStaticMeshComponent) "ECC_PhysicsBody")
  (Collision|SetCollisionResponsetoChannel (Variables|Debug|GetStaticMeshComponent) "ECC_Pawn" "ECR_Block")
  (Variables|Default|SetLocationAlpha 0.0))

(fn IsValidHit
  (params (Actor :type Actor%20Object%20Reference))
  (LocalVariables|SetHitValid true)
  (for _array_element (Variables|Default|GetActorToIgnore)
    (if (== _array_element Actor)
      ;[1 1 1] ?????????????????????????????
      (Variables|Default|SetIsGrabbed false)))
  (return (LocalVariables|GetHitValid)))

(fn DropifLostConnection
  (bind _mc (Variables|Default|GetMC))
  (Utilities|IsValid _mc
    (:Is%20Valid
      (if (> (Math|Vector|VectorLength (- (Transformation|GetWorldLocation (Variables|Default|GetPivot)) (Transformation|GetWorldLocation _mc))) (Variables|Default|GetDisconnectionDistance))
        (CallFunction|Drop))
      (return))))

(fn IsHeldbyMe
  (params (MC :type Scene%20Component%20Object%20Reference))
  (return (== MC (Variables|Default|GetMC))))