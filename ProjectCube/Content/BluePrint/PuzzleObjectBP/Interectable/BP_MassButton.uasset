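; BP_MassButton is an interactable puzzle button that switches connected actors on and off.
; When its Pad component begins or ends overlapping the Box trigger, it sends true or false to each ConnectedActor implementing BI_SendMessage.
; Only the Pad triggers it, so the state follows the pad's position rather than whatever touches the box.
; The construction script draws brief debug lines to valid connected actors to visualize the links.
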(event OnComponentBeginOverlap(Box)
  (params (OverlappedComponent :type Primitive%20Component%20Object%20Reference) (OtherActor :type Actor%20Object%20Reference) (OtherComp :type Primitive%20Component%20Object%20Reference) (OtherBodyIndex :type Integer) (bFromSweep :type Boolean) (SweepResult :type Hit%20Result%20Structure%20%28by%20ref%29))
  (if (== OtherComp (Variables|Default|GetPad))
    (for _array_element (Variables|Default|GetConnectedActor)
      (if (Utilities|DoesObjectImplementInterface _array_element "/Game/BluePrint/PuzzleObjectBP/BI_SendMessage.BI_SendMessage_C")
        (Class|BISendMessage|SendMessage(Message) _array_element true)))))

(event OnComponentEndOverlap(Box)
  (params (OverlappedComponent :type Primitive%20Component%20Object%20Reference) (OtherActor :type Actor%20Object%20Reference) (OtherComp :type Primitive%20Component%20Object%20Reference) (OtherBodyIndex :type Integer))
  (if (== OtherComp (Variables|Default|GetPad))
    (for _array_element (Variables|Default|GetConnectedActor)
      (if (Utilities|DoesObjectImplementInterface _array_element "/Game/BluePrint/PuzzleObjectBP/BI_SendMessage.BI_SendMessage_C")
        (Class|BISendMessage|SendMessage(Message) _array_element false)))))

(event EventBeginPlay)

(event Collision|EventActorBeginOverlap
  (params (OtherActor :type Actor%20Object%20Reference)))

(event EventTick
  (params (DeltaSeconds :type Float%20%28single-precision%29)))

(fn ConstructionScript
  (for _array_element (Variables|Default|GetConnectedActor)
    (Utilities|IsValid _array_element
      (:Is%20Valid
        (Rendering|Debug|DrawDebugLine (Transformation|GetActorLocation) (Transformation|GetActorLocation _array_element) "(R=1.000000,G=0.047119,B=0.000000,A=1.000000)" 0.1 5.0)))))