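; Grabbable puzzle laser emitter that fires a red, green or blue beam, bouncing off reflective surfaces to trigger sensors.
; BeginPlay pools one beam actor per allowed bounce, and the construction script tints the arrow to match the color.
; Tick, after a short delay, runs CastLight: it resets the last sensor and beams, then line-traces segments, mirroring at reflectors.
; Reflectors and sensors are identified by hit-face material, and sensors receive the laser color.
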(event EventTick
  (params (DeltaSeconds :type Float%20%28single-precision%29))
  (bind _arrow (Variables|Default|GetArrow))
  (|CallParentFunction DeltaSeconds)
  (Utilities|FlowControl|Delay 0.01)
  (CallFunction|CastLight (Transformation|GetWorldLocation _arrow) (Math|Vector|GetForwardVector _arrow) (Variables|Default|GetCastDistance)))

(event EventBeginPlay
  (|CallParentFunction)
  (Utilities|FlowControl|Sequence
    (:then_0
      (switch Utilities|FlowControl|Switch|SwitchonE_LaserColor (Variables|Default|GetLaserColor)
        (:NewEnumerator0
          (Variables|Default|SetColor "(R=1.000000,G=0.000000,B=0.000000,A=1.000000)"))
        (:NewEnumerator1
          (Variables|Default|SetColor "(R=0.000000,G=1.000000,B=0.000000,A=1.000000)"))
        (:NewEnumerator2
          (Variables|Default|SetColor "(R=0.000000,G=0.000000,B=1.000000,A=1.000000)"))))
    (:then_1
      (Utilities|Array|Clear (Variables|Default|GetBeams))
      (for _index (range 0 (- (Variables|Default|GetMaxReflectionNum) 1))
        (bind _returnvalue (Game|SpawnActorfromClass "/Game/BluePrint/PuzzleObjectBP/Laser/LaserBeam.LaserBeam_C" (Math|Transform|MakeTransform "0, 0, 0" "0, 0, 0" "0.010000,0.010000,0.010000") "Undefined" 0 0))
        (Utilities|Array|Add (Variables|Default|GetBeams) _returnvalue)))))

(fn ConstructionScript
  (switch Utilities|FlowControl|Switch|SwitchonE_LaserColor (Variables|Default|GetLaserColor)
    (:NewEnumerator0
      (Variables|/Script/Engine.ArrowComponent|SetArrowColor (Variables|Default|GetArrow) (Math|Conversions|ToColor(LinearColor) "(R=1.000000,G=0.000000,B=0.000000,A=1.000000)")))
    (:NewEnumerator1
      (Variables|/Script/Engine.ArrowComponent|SetArrowColor (Variables|Default|GetArrow) (Math|Conversions|ToColor(LinearColor) "(R=0.118336,G=1.000000,B=0.000000,A=1.000000)")))
    (:NewEnumerator2
      (Variables|/Script/Engine.ArrowComponent|SetArrowColor (Variables|Default|GetArrow) (Math|Conversions|ToColor(LinearColor) "(R=0.000000,G=0.000000,B=1.000000,A=1.000000)")))
    (:NewEnumerator3
      (Development|PrintString "Emitter은 ACtionEveryColor로 설정할 수 없습니다."))))

(fn CastLight
  (params (CastOrigin :type Vector) (CastDirection :type Vector) (CastDistance :type Float%20%28single-precision%29))
  ;[1 1 1] Init
  (LocalVariables|SetL_CastOrigin CastOrigin)
  (LocalVariables|SetL_CastDirection CastDirection)
  (LocalVariables|SetL_CastDistance CastDistance)
  (Class|BISendMessage|SendMessageColor(Message) (Variables|Default|GetActivatedSensor) false (Variables|Default|GetLaserColor))
  (for _array_element (Variables|Default|GetBeams)
    (Default|SetVisible _array_element false))
  (LocalVariables|SetL_WhileIndex -1)
  (while (LocalVariables|GetL_Continue)
    (LocalVariables|SetL_WhileIndex (+ (LocalVariables|GetL_WhileIndex) 1))
    (Utilities|FlowControl|Sequence
      (:then_0
        (bind (_outhit _returnvalue) (Collision|LineTraceByChannel (LocalVariables|GetL_CastOrigin) (+ (LocalVariables|GetL_CastOrigin) (* (LocalVariables|GetL_CastDirection) (LocalVariables|GetL_CastDistance))) "TraceTypeQuery3" true 0 "None" false "(R=1.000000,G=0.000000,B=0.000000,A=1.000000)" "(R=0.000000,G=1.000000,B=0.000000,A=1.000000)" 0.1))
        (LocalVariables|SetL_BeamStart (LocalVariables|GetL_CastOrigin))
        ;[1 1 1] Is hit?
        (if _returnvalue
          (LocalVariables|SetL_BeamEnd (.ImpactPoint (Collision|BreakHitResult _outhit)))
          ;[1 1 1] Is Hit Reflector?
          (if (== (Variables|Default|GetReflectMaterial) (.ReturnValue (Class|PrimitiveComponent|GetMaterialfromCollisionFaceIndex (.HitComponent (Collision|BreakHitResult _outhit)) (.FaceIndex (Collision|BreakHitResult _outhit)))))
            (LocalVariables|SetL_CastOrigin (.ImpactPoint (Collision|BreakHitResult _outhit)))
            (LocalVariables|SetL_CastDirection (Math|Vector|MirrorVectorbyNormal (LocalVariables|GetL_CastDirection) (.ImpactNormal (Collision|BreakHitResult _outhit))))
            (LocalVariables|SetL_Continue true)
            (else
              (bind _asmaterial_instance (Utilities|Casting|CastToMaterialInstance (.ReturnValue (Class|PrimitiveComponent|GetMaterialfromCollisionFaceIndex (.HitComponent (Collision|BreakHitResult _outhit)) (.FaceIndex (Collision|BreakHitResult _outhit)))))
                (:then
                  _)
                (:CastFailed
                  _))
              ;[1 1 1] Is Hit Sensor??
              (if (or (== (.ReturnValue (Class|PrimitiveComponent|GetMaterialfromCollisionFaceIndex (.HitComponent (Collision|BreakHitResult _outhit)) (.FaceIndex (Collision|BreakHitResult _outhit)))) (Variables|Default|GetSensorMaterial)) (== _asmaterial_instance (Variables|Default|GetSensorMaterialInst)))
                (Class|BISendMessage|SendMessageColor(Message) (.HitActor (Collision|BreakHitResult _outhit)) true (Variables|Default|GetLaserColor))
                (Variables|Default|SetActivatedSensor (.HitActor (Collision|BreakHitResult _outhit)))
                ;[1 1 1] Stop Trace
                (LocalVariables|SetL_Continue false)
                (else
                  (LocalVariables|SetL_Continue false)))))
          (else
            (LocalVariables|SetL_BeamEnd (+ (LocalVariables|GetL_CastOrigin) (* (LocalVariables|GetL_CastDirection) (LocalVariables|GetL_CastDistance))))
            (LocalVariables|SetL_Continue false))))
      (:then_1
        ;[1 1 1] 개수제한
        (if (>= (+ (LocalVariables|GetL_WhileIndex) 1) (Variables|Default|GetMaxReflectionNum))
          (LocalVariables|SetL_Continue false)))
      (:then_2
        (Default|SetVisible (Utilities|Array|Get(acopy) (Variables|Default|GetBeams) (LocalVariables|GetL_WhileIndex)) true)
        (Default|DrawLaser (Utilities|Array|Get(acopy) (Variables|Default|GetBeams) (LocalVariables|GetL_WhileIndex)) (LocalVariables|GetL_BeamStart) (LocalVariables|GetL_BeamEnd) (Variables|Default|GetColor))))))