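; A fixed laser sensor puzzle object that switches connected actors on or off in response to color messages.
; SendMessageColor accepts only CorrectColor, or any color when set to the sensor-only wildcard, then stores State and relays it to each ConnectedActor through SendMessageMessage.
; The construction script draws brief debug lines to connected actors and tints the Arrow to match a red, green or blue CorrectColor.
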(event EventSendMessageColor
  (params (On :type Boolean) (Color :type E_LaserColor%20Enum :default "NewEnumerator0"))
  (bind _correctcolor (Variables|Default|GetCorrectColor))
  (if (Utilities|Enum|Equal(Enum) Color _correctcolor)
    (if On :!label _label
      (Variables|Default|SetState true)
      (for _array_element (Variables|Default|GetConnectedActor)
        (Class|BISendMessage|SendMessage(Message) _array_element true))
      (else
        (Variables|Default|SetState false)
        (for _array_element_2 (Variables|Default|GetConnectedActor)
          (Class|BISendMessage|SendMessage(Message) _array_element_2 false))))
    (elif (Utilities|Enum|Equal(Enum) _correctcolor "NewEnumerator3")
      (goto _label))))

(fn ConstructionScript
  (Utilities|FlowControl|Sequence
    (:then_0
      (for _array_element (Variables|Default|GetConnectedActor)
        (Utilities|IsValid _array_element
          (:Is%20Valid
            (Rendering|Debug|DrawDebugLine (Transformation|GetActorLocation) (Transformation|GetActorLocation _array_element) "(R=1.000000,G=0.047119,B=0.000000,A=1.000000)" 0.1 5.0)))))
    (:then_1
      (switch Utilities|FlowControl|Switch|SwitchonE_LaserColor (Variables|Default|GetCorrectColor)
        (:NewEnumerator0
          (Variables|/Script/Engine.ArrowComponent|SetArrowColor (Variables|Default|GetArrow) (Math|Conversions|ToColor(LinearColor) "(R=1.000000,G=0.000000,B=0.000000,A=1.000000)")))
        (:NewEnumerator1
          (Variables|/Script/Engine.ArrowComponent|SetArrowColor (Variables|Default|GetArrow) (Math|Conversions|ToColor(LinearColor) "(R=0.118336,G=1.000000,B=0.000000,A=1.000000)")))
        (:NewEnumerator2
          (Variables|/Script/Engine.ArrowComponent|SetArrowColor (Variables|Default|GetArrow) (Math|Conversions|ToColor(LinearColor) "(R=0.000000,G=0.000000,B=1.000000,A=1.000000)")))))))