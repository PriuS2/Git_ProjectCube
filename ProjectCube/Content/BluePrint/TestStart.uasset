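; TestStart is a Blueprint that picks which pawn the player controls, a first-person character or a VR one, apparently for testing.
; On BeginPlay, the PossessFirstPersonCharacter flag decides whether player controller 0 possesses the FP or the VR reference.
; Any key press makes that controller possess FP, regardless of the flag.
; The overlap, Tick and construction script graphs are empty.
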(event EventBeginPlay
  (bind _returnvalue (Game|GetPlayerController 0))
  (if (Variables|Default|GetPossessFirstPersonCharacter)
    (Pawn|Possess _returnvalue (Variables|Default|GetFP))
    (else
      (Pawn|Possess _returnvalue (Variables|Default|GetVR)))))

(event Collision|EventActorBeginOverlap
  (params (OtherActor :type Actor%20Object%20Reference)))

(event EventTick
  (params (DeltaSeconds :type Float%20%28single-precision%29)))

(event Input|KeyboardEvents|AnyKey
  (params (Key :type Key%20Structure :default "None"))
  (:Pressed
    (Pawn|Possess (Game|GetPlayerController 0) (Variables|Default|GetFP))))

(fn ConstructionScript)